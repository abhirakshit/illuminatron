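; RefractionMath is a set of math functions in the Dynamic Laser System that computes how a direction vector bends between two refractive indices.
; Refract compares the incidence angle to the critical angle from SnellCritical, returning a reflection above it and a vector along the surface at it.
; Below it, SnellAngle supplies the Snell's law angle, used to build the outgoing direction from the surface tangent and inverted normal.
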(fn `Refract`
  (params (Direction :type "Vector Structure") (Normal :type "Vector Structure") (IndexFrom :type "Float (double-precision)") (IndexTo :type "Float (double-precision)"))
  (returns (Refracted :type "Vector Structure"))
  (locals (angle1 :type "Float (double-precision)") (angle2 :type "Float (double-precision)") (dot :type "Float (double-precision)") (result :type "Vector Structure"))
  (bind _returnvalue (`KismetMathLibrary.GetReflectionVector` Direction Normal))
  (bind _angle2 (`local.angle2`))
  (bind _dot (`local.dot`))
  (bind _returnvalue_2 (- _returnvalue (* Normal (`local.dot`))))
  (bind _returnvalue_3 (`KismetMathLibrary.Normal` (+ (* _returnvalue_2 (`KismetMathLibrary.Sin` _angle2)) (* Normal (* (`KismetMathLibrary.Cos` _angle2) -1.0)))))
  (bind _output_get (set `local.dot` (`KismetMathLibrary.Dot_VectorVector` (* Direction -1.0) Normal)))
  (bind _output_get_2 (set `local.angle1` (`KismetMathLibrary.Acos` _output_get)))
  (`/Engine/EditorBlueprintResources/StandardMacros.CompareFloat` _output_get_2 (`self.SnellCritical` IndexFrom IndexTo)
    (:`>`
      ;[1 1 1] When angle > critical, there is no refraction, only reflection
      (return _returnvalue))
    (:`==`
      ;[1 1 1] When angle = critical, there is no refraction nor reflection
      (return (`KismetMathLibrary.Normal` _returnvalue_2)))
    (:`<`
      (set `local.angle2` (`self.SnellAngle` _output_get_2 IndexFrom IndexTo))
      (if (!= (`local.dot`) 0.0)
        ;[1 1 1] When angle < critical, there is refraction
        (return _returnvalue_3)
        (else
          (return (* _returnvalue_3 (/ _dot (`KismetMathLibrary.Abs` _dot)))))))))

(fn `SnellAngle`
  (params (angle1 :type "Float (double-precision)") (index1 :type "Float (double-precision)") (index2 :type "Float (double-precision)"))
  (returns (angle2 :type "Float (double-precision)"))
  (return (`KismetMathLibrary.Asin` (* (`KismetMathLibrary.Sin` angle1) (/ index1 index2)))))

(fn `SnellCritical`
  (params (index1 :type "Float (double-precision)") (index2 :type "Float (double-precision)"))
  (returns (criticalAngle :type "Float (double-precision)"))
  (return (`KismetMathLibrary.Asin` (/ index2 index1))))