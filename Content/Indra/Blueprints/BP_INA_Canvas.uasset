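; Paintable canvas actor that shows the RT_INA_Canvas render target on its mesh through a dynamic shell material, clearing it at BeginPlay.
; Three draw variants stamp a dynamic brush material into render targets: by channel, by color, or by texture and size.
; The textured variant uses canvas drawing and adds a second stamp near edges to wrap around.
; A looping timer and gate periodically invert the target opacity, which Tick eases toward on the shell.
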(event Custom|OpenGate
  (Utilities|FlowControl|Gate true) ; enters at Open
)

(event Custom|CloseGate
  (Utilities|FlowControl|Gate true) ; enters at Close
)

(event EventBeginPlay
  (Utilities|FlowControl|Sequence
    (:then_0
      (bind _returnvalue (Rendering|Material|CreateDynamicMaterialInstance "/Game/Indra/Materials/Finished/M_Brush.M_Brush" "None" :!class /Script/Engine.KismetMaterialLibrary))
      (bind _output_get (Variables|Default|Setbrush _returnvalue))
      (CallFunction|GetINAPawn))
    (:then_1
      (bind _returnvalue_2 (Rendering|Material|CreateDynamicMaterialInstance "/Game/Indra/Materials/Finished/M_Shell.M_Shell" "None" :!class /Script/Engine.KismetMaterialLibrary))
      (bind _output_get_2 (Variables|Default|SetShell%20Material _returnvalue_2))
      (bind _output_get_3 (Variables|Default|SetCanvas "/Game/Indra/Materials/Finished/RT_INA_Canvas.RT_INA_Canvas"))
      (Rendering|Material|SetTextureParameterValue _output_get_2 "RenderTarget" _output_get_3)
      (Rendering|Material|SetMaterial (Variables|Default|GetStaticMesh) 0 _output_get_2))
    (:then_2
      (Rendering|ClearRenderTarget2D "/Game/Indra/Materials/Finished/RT_INA_Canvas.RT_INA_Canvas"))
    (:then_3
      (Utilities|Time|SetTimerbyEvent (delegate Custom|OpenGate) 5.0 true))))

(event EventTick
  (params (DeltaSeconds :type Float%20%28single-precision%29))
  (Utilities|FlowControl|Sequence
    (:then_0
      (Utilities|FlowControl|Gate true
        (:Exit
          (CallFunction|CloseGate)
          (if (Math|Float|NearlyEqual(Float) (Variables|Default|Getcurrent%20opacity) (Variables|Default|Getopacity) 0.1)
            (Variables|Default|Setopacity (- 1.0 (Variables|Default|Getopacity)))))))
    (:then_1
      (bind _output_get (Variables|Default|Setcurrent%20opacity (Math|Float|Lerp (Variables|Default|Getcurrent%20opacity) (Variables|Default|Getopacity) 0.133)))
      (Rendering|Material|SetScalarParameterValue (Variables|Default|GetShell%20Material) "Opacity" _output_get :!class /Script/Engine.MaterialInstanceDynamic))))

(fn ConstructionScript)

(fn DrawonSurface
  (params (position :type Vector%202D%20Structure) (color :type Color%20Structure))
  (bind (_b _g _r) (Math|Color|BreakColor color))
  (bind _returnvalue (Math|Conversions|ToVector(Vector2D) position))
  (bind _brush (Variables|Default|Getbrush))
  (bind _returnvalue_2 (Math|Conversions|ToLinearColor(Vector) _returnvalue))
  (Utilities|FlowControl|Sequence
    (:then_1
      (Rendering|Material|SetScalarParameterValue _brush "Alpha" (Math|Conversions|ToFloat(Byte) _b) :!class /Script/Engine.MaterialInstanceDynamic)
      (Rendering|Material|SetVectorParameterValue _brush "Position" _returnvalue_2 :!class /Script/Engine.MaterialInstanceDynamic)
      (LocalVariables|SetRenderTarget "/Game/Indra/Materials/Finished/RT_INA_Canvas.RT_INA_Canvas")
      (Rendering|Material|SetTextureParameterValue _brush "RenderTarget" (LocalVariables|GetRenderTarget))
      (Rendering|DrawMaterialtoRenderTarget (LocalVariables|GetRenderTarget) _brush))
    (:then_2
      (Rendering|Material|SetScalarParameterValue _brush "Alpha" (Math|Conversions|ToFloat(Byte) _g) :!class /Script/Engine.MaterialInstanceDynamic)
      (Rendering|Material|SetVectorParameterValue _brush "Position" _returnvalue_2 :!class /Script/Engine.MaterialInstanceDynamic)
      (LocalVariables|SetRenderTarget 0)
      (Rendering|Material|SetTextureParameterValue _brush "RenderTarget" (LocalVariables|GetRenderTarget))
      (Rendering|DrawMaterialtoRenderTarget (LocalVariables|GetRenderTarget) _brush))
    (:then_3
      (Rendering|Material|SetScalarParameterValue _brush "Alpha" (Math|Conversions|ToFloat(Byte) _r) :!class /Script/Engine.MaterialInstanceDynamic)
      (Rendering|Material|SetVectorParameterValue _brush "Position" _returnvalue_2 :!class /Script/Engine.MaterialInstanceDynamic)
      (LocalVariables|SetRenderTarget 0)
      (Rendering|Material|SetTextureParameterValue _brush "RenderTarget" (LocalVariables|GetRenderTarget))
      (Rendering|DrawMaterialtoRenderTarget (LocalVariables|GetRenderTarget) _brush))))

(fn DrawonSurface2
  (params (position :type Vector%202D%20Structure) (color :type Linear%20Color%20Structure))
  (bind _brush (Variables|Default|Getbrush))
  (Rendering|Material|SetVectorParameterValue _brush "Color" color :!class /Script/Engine.MaterialInstanceDynamic)
  (Rendering|Material|SetVectorParameterValue _brush "Position" (Math|Conversions|ToLinearColor(Vector) (Math|Conversions|ToVector(Vector2D) position)) :!class /Script/Engine.MaterialInstanceDynamic)
  (bind _output_get (LocalVariables|SetRenderTarget "/Game/Indra/Materials/Finished/RT_INA_Canvas.RT_INA_Canvas"))
  (Rendering|Material|SetTextureParameterValue _brush "RenderTarget" _output_get)
  (Rendering|DrawMaterialtoRenderTarget _output_get _brush))

(fn DrawonSurface3
  (params (texture :type Texture%202D%20Object%20Reference) (position :type Vector%202D%20Structure) (brush%20size :type Float%20%28single-precision%29))
  (bind _returnvalue (Class|KismetSystemLibrary|MakeLiteralBool false))
  (bind _brush (Variables|Default|Getbrush))
  (LocalVariables|SetlocBrushSize (Math|Float|Clamp(Float) brush%20size 3.0 128.0))
  (Utilities|FlowControl|Sequence
    (:then_0
      (Rendering|Material|SetTextureParameterValue (Variables|Default|Getbrush) "BrushTexture" texture))
    (:then_1
      (bind (_canvas _size _context) (Rendering|BeginDrawCanvastoRenderTarget (LocalVariables|GetRenderTarget)))
      (LocalVariables|SetCanvasSize _size)
      (bind _output_get (LocalVariables|SetPositionOnCanvas (- (* _size position) (/ (LocalVariables|GetlocBrushSize) 2.0))))
      (LocalVariables|Setx2 (.x _output_get))
      (LocalVariables|Sety2 (.y _output_get))
      ;[1 1 1] Lower Bound
      (if (<= (.x (- (LocalVariables|GetPositionOnCanvas) (/ (LocalVariables|GetlocBrushSize) 2.0))) 0.0)
        (LocalVariables|Setx2 (+ (.x (LocalVariables|GetCanvasSize)) (* (.x (- (LocalVariables|GetPositionOnCanvas) (/ (LocalVariables|GetlocBrushSize) 2.0))) 0.5))))
      (if (<= (.y (- (LocalVariables|GetPositionOnCanvas) (/ (LocalVariables|GetlocBrushSize) 2.0))) 0.0)
        (LocalVariables|Sety2 (+ (.y (LocalVariables|GetCanvasSize)) (* (.y (- (LocalVariables|GetPositionOnCanvas) (/ (LocalVariables|GetlocBrushSize) 2.0))) 0.5))))
      ;[1 1 1] Upper Bound
      (if (>= (.x (+ (LocalVariables|GetPositionOnCanvas) (LocalVariables|GetlocBrushSize))) (.x (LocalVariables|GetCanvasSize)))
        (bind _output_get_2 (LocalVariables|Setx2 (- (* (.x (+ (LocalVariables|GetPositionOnCanvas) (LocalVariables|GetlocBrushSize))) (|(1-((BrushSize/100)*0.095000)) (LocalVariables|GetlocBrushSize))) (.x (LocalVariables|GetCanvasSize)))))
        (Development|PrintString (Utilities|String|Append "X2: " (Utilities|String|ToString(Float) _output_get_2)) _returnvalue _returnvalue))
      (if (>= (.y (+ (LocalVariables|GetPositionOnCanvas) (LocalVariables|GetlocBrushSize))) (.y (LocalVariables|GetCanvasSize)))
        (bind _output_get_3 (LocalVariables|Sety2 (- (* (.y (+ (LocalVariables|GetPositionOnCanvas) (LocalVariables|GetlocBrushSize))) (|(1-((BrushSize/100)*0.095000)) (LocalVariables|GetlocBrushSize))) (.y (LocalVariables|GetCanvasSize)))))
        (Development|PrintString (Utilities|String|Append "Y2: " (Utilities|String|ToString(Float) _output_get_3)) _returnvalue _returnvalue))
      (Canvas|DrawMaterial :self _canvas :RenderMaterial _brush :ScreenPosition (- (* _size position) (/ (LocalVariables|GetlocBrushSize) 2.0)) :ScreenSize (Math|Vector2D|MakeVector2D (LocalVariables|GetlocBrushSize) (LocalVariables|GetlocBrushSize)))
      (if (or (!= (Math|Float|Floor (LocalVariables|Getx2)) (Math|Float|Floor (.x (LocalVariables|GetPositionOnCanvas)))) (!= (Math|Float|Floor (LocalVariables|Gety2)) (Math|Float|Floor (.y (LocalVariables|GetPositionOnCanvas)))))
        (Canvas|DrawMaterial :self _canvas :RenderMaterial _brush :ScreenPosition (Math|Vector2D|MakeVector2D (LocalVariables|Getx2) (LocalVariables|Gety2)) :ScreenSize (Math|Vector2D|MakeVector2D (LocalVariables|GetlocBrushSize) (LocalVariables|GetlocBrushSize)) :PivotPoint "(X=0.500000,Y=0.500000)"))
      (Rendering|EndDrawCanvastoRenderTarget _context)
      (Development|PrintString "" _returnvalue _returnvalue))))