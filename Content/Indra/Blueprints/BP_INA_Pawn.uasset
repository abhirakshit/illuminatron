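; Player pawn for Indra that carries a procedural shell mesh and a camera boom, and fires BP_Laser projectiles.
; BeginPlay builds the noisy runtime shell with a dynamic material fed by a canvas render target (unless DisableMesh), then registers it with the controller and refreshes HUD vessel sliders.
; Each Tick, the authority passes actor and boom transforms through SmoothClient events that apply them directly, without interpolation.
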(event `self.ReceiveBeginPlay`
  (`parent.ReceiveBeginPlay`)
  (if (`self.DisableMesh`)
    (bind _asina_pawn_controller (`/Game/Indra/Functions/Basic_Library.Get INA Controller for Pawn` self :!label _label))
    (`INA_PawnController.SetSelectedShell` _asina_pawn_controller (`self.ShellComponent`))
    (bind _asbp_ina_pawn_controller (cast `/Game/Indra/Blueprints/BP_INA_PawnController` _asina_pawn_controller))
    (`/Game/Indra/GUI/HUD.Update Vessel Sliders` (`/Game/Indra/Blueprints/BP_INA_PawnController.TheHUD` _asbp_ina_pawn_controller))
    (else
      (`|ExecutionSequence`
        (:`then_0`
          (`self.Create Shell Mesh` (`self.ShellComponent`)))
        (:`then_1`
          (goto _label))))))

(event `self.ReceiveTick`
  (params (DeltaSeconds :type "Float (single-precision)"))
  (`self.SmoothClient`))

(event `SmoothClientBoomTransform`
  (params (Transform :type "Transform Structure"))
  (`SceneComponent.K2_SetWorldTransform` (`self.CameraRotatorArm`) Transform false false))

(event `SmoothClientTransform`
  (params (Transform :type "Transform Structure"))
  (`self.K2_SetActorTransform` Transform))

(fn `Create Shell Mesh`
  (params (Shell :type "ShellComponent Object Reference"))
  (locals (`Shell In` :type "ShellComponent Object Reference"))
  (bind _shell_in (`local.Shell In`))
  (set `local.Shell In` Shell)
  (`self.SetShellProperties` (`local.Shell In`) (`self.Subdivisions`) 100.0 0.1)
  (`|ExecutionSequence`
    (:`then_0`
      (`ShellComponent.CreateRuntimeComponents` _shell_in)
      (`ShellComponent.CreateMeshSection` _shell_in))
    (:`then_1`
      ;[1 1 1] Material
      (bind _returnvalue (`KismetMaterialLibrary.CreateDynamicMaterialInstance` "/Game/Indra/Materials/Finished/M_Shell.M_Shell"))
      (`|ExecutionSequence`
        (:`then_0`
          (`ShellComponent.SetMeshMaterial` (`local.Shell In`) _returnvalue))
        (:`then_1`
          ;;[1 1 1] All shells will probably share the same canvas RT
          (`MaterialInstanceDynamic.SetTextureParameterValue` _returnvalue "RenderTarget" "/Game/Indra/Materials/Finished/RT_INA_Canvas.RT_INA_Canvas"))))))

(fn `SmoothClient`
  (`/Engine/EditorBlueprintResources/ActorMacros.Switch Has Authority`
    (:`Authority`
      (`self.SmoothClientBoomTransform` (`SceneComponent.K2_GetComponentToWorld` (`self.CameraRotatorArm`)))
      (`self.SmoothClientTransform` (`self.GetTransform`)))))

(fn `UserConstructionScript`
  (`self.SetLaserProjectileType` "/Game/Indra/Blueprints/Lasers/BP_Laser.BP_Laser_C"))