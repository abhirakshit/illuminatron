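; BP_INA_PawnController is a player controller that owns the HUD and switches input modes.
; On BeginPlay it creates the HUD widget and adds it to the viewport.
; The CursorMode action toggles a mode enum, showing the mouse cursor when Movement switches to HUD cursor and hiding it when Placement or HUD cursor returns to Movement.
; The EscapeKey action quits the game.
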(event `self.ReceiveBeginPlay`
  (bind _returnvalue (`|CreateWidget` "/Game/Indra/GUI/HUD.HUD_C" self))
  (bind _output_get (set `self.TheHUD` _returnvalue))
  (`UserWidget.AddToViewport` _output_get 0))

(event `InputAction|CursorMode`
  (params (Key :type "Key Structure"))
  (:`Pressed`
    (switch `ControllerMode` (`self.Mode`)
      (:`Movement`
        (set `self.bShowMouseCursor` true)
        (set `self.Mode` "HUDCursor"))
      (:`Placement`
        (set `self.bShowMouseCursor` false :!label _label)
        (set `self.Mode` "Movement"))
      (:`HUDCursor`
        (goto _label)))))

(event `InputAction|EscapeKey`
  (params (Key :type "Key Structure"))
  (:`Pressed`
    (`KismetSystemLibrary.QuitGame` null "Quit")))

(fn `UserConstructionScript`)